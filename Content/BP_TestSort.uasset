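; BP_TestSort is a test Blueprint for a compute shader that sorts entries, judging by its name and debug output.
; It passes an array variable and its length as the particle count to the asynchronous ExecuteBaseComputeShader node on BeginPlay and again every Tick.
; On completion it prints each returned entry and offset, with a label after each list.
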(event `self.ReceiveBeginPlay`
  (bind _newvar (`self.NewVar`))
  (bind (_entries _offsets) (`GPUSortLibrary_AsyncExecution.ExecuteBaseComputeShader` _newvar (`KismetArrayLibrary.Array_Length` _newvar) :!label _label)
    (:`Completed`
      (for _array_element _entries
        (`KismetSystemLibrary.PrintString` (`KismetStringLibrary.Conv_IntVectorToString` _array_element)))
      (`KismetSystemLibrary.PrintString` "Entries Sorted")
      (for _array_element_2 _offsets
        (`KismetSystemLibrary.PrintString` (`KismetStringLibrary.Conv_IntToString` _array_element_2)))
      (`KismetSystemLibrary.PrintString` "offsets"))))

(event `self.ReceiveTick`
  (params (DeltaSeconds :type "Float (single-precision)"))
  (goto _label))

(fn `UserConstructionScript`)